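; Player character for a sword-combat game, handling health, attack animations and respawn-style repositioning against an AI enemy.
; On BeginPlay it sets game-only input, loops the MusicLights sequence and caches the enemy; slash and block events play montages.
; Damage drains health until the player controller's OnDeath fires, while Freeze and Unfreeze toggle walk speed.
; TeleportPlayer picks a random index for paired spawn arrays, moving the player, then spawning an enemy after a delay.
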(event `self.ReceiveBeginPlay`
  (`WidgetBlueprintLibrary.SetInputMode_GameOnly` (`GameplayStatics.GetPlayerController` 0))
  (`LevelSequencePlayer.CreateLevelSequencePlayer` "/Game/Level/Sequence/MusicLights.MusicLights" (make `MovieSceneSequencePlaybackSettings` true (make `MovieSceneSequenceLoopCount` 100000)))
  (bind _returnvalue (`GameplayStatics.GetActorOfClass` "/Game/AI/BP_AICharacter.BP_AICharacter_C"))
  (set `self.enemyPawn` _returnvalue))

(event `CustomEvent`
  (params (Damage :type Integer))
  (bind _output_get (set `self.Health` (- (`self.Health`) Damage)))
  (if (<= _output_get 0)
    (bind _asbp_to_the_edge_player_controller (cast `/Game/BP_ToTheEdgePlayerController` (`self.GetController`)))
    (`/Game/BP_ToTheEdgePlayerController.OnDeath` _asbp_to_the_edge_player_controller)))

(event `OverheadSlash`
  (`|PlayMontage` (`self.MainMesh`) "/Game/Assets/Character/Models/Montage/OVerhead-SwordSlash.OVerhead-SwordSlash"))

(event `Right-Slash`
  (`|PlayMontage` (`self.MainMesh`) "/Game/Assets/Character/Models/Montage/Right-Sword-Slash.Right-Sword-Slash"))

(event `left-Slash`
  (`|PlayMontage` (`self.MainMesh`) "/Game/Assets/Character/Models/Montage/Left-SwordSlash.Left-SwordSlash"))

(event `Block`
  (`|PlayMontage` (`self.MainMesh`) "/Game/Assets/Character/Models/Montage/Sword-Block.Sword-Block"))

(event `Freeze`
  (set `CharacterMovementComponent.MaxWalkSpeed` 0.0 (`self.CharacterMovement`)))

(event `Unfreeze`
  (set `CharacterMovementComponent.MaxWalkSpeed` 200.0 (`self.CharacterMovement`)))

(event `TeleportPlayer`
  (bind _output_get (set `self.SpawnLocation` (`KismetMathLibrary.RandomInteger` 3)))
  (`self.K2_TeleportTo` (`|GetArrayItem` (`self.PlayerSpawns`) _output_get))
  (`KismetSystemLibrary.Delay` 4.0)
  (`AIBlueprintHelperLibrary.SpawnAIFromClass` "/Game/AI/BP_AICharacter.BP_AICharacter_C" "/Game/AI/BT_AICharacter.BT_AICharacter" (`|GetArrayItem` (`self.AISpawns`) _output_get) (struct) false null)
  (`GameplayStatics.PlaySoundAtLocation` "/Game/Assets/Audio/enemy-spawning_Cue.enemy-spawning_Cue" (0.0 0.0 0.0) (struct) 0.5 1.0 0.0 null null null))

(fn `UserConstructionScript`)