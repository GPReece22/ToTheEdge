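; AI enemy character for sword combat, with events that play slash, block and parry-impact montages and a setter for walk speed.
; Any actor that begins overlapping it is sent a 10-damage message.
; AttackLeft sends a left-attack notification to the cached player controller and sets a timer on it with no function name.
; The parry-or-damage check against the controller's block flag and health is left unconnected and never runs.
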(event `self.ReceiveBeginPlay`
  (bind _asbp_to_the_edge_player_controller (cast `/Game/BP_ToTheEdgePlayerController` (`GameplayStatics.GetPlayerController` 0)))
  (set `self.PlayerControllerReference` _asbp_to_the_edge_player_controller))

(event `self.ReceiveActorBeginOverlap`
  (params (OtherActor :type "Actor Object Reference"))
  (message `/Game/BPI_Damage.Take Damage` OtherActor 10))

(event `OverheadSlash`
  (`|PlayMontage` (`self.Mesh`) "/Game/Assets/Character/Models/Montage/OVerhead-SwordSlash.OVerhead-SwordSlash"))

(event `Right-Slash`
  (`|PlayMontage` (`self.Mesh`) "/Game/Assets/Character/Models/Montage/Right-Sword-Slash.Right-Sword-Slash"))

(event `LeftSlash`
  (`|PlayMontage` (`self.Mesh`) "/Game/Assets/Character/Models/Montage/Left-SwordSlash.Left-SwordSlash"))

(event `ParryImpact`
  (`|PlayMontage` (`self.Mesh`) "/Game/Assets/Character/Models/Montage/ParryImpact.ParryImpact"))

(event `Sword-Block`
  (`|PlayMontage` (`self.Mesh`) "/Game/Assets/Character/Models/Montage/Sword-Block.Sword-Block"))

(fn `AttackLeft`
  (bind _playercontrollerreference (`self.PlayerControllerReference`))
  (`/Game/BP_ToTheEdgePlayerController.LeftNotification` _playercontrollerreference)
  (bind _returnvalue (`KismetSystemLibrary.K2_SetTimer` _playercontrollerreference "" 5.0)))

(fn `UpdateWalkSpeed`
  (params (NewWalkSpeed :type "Float (double-precision)"))
  (set `CharacterMovementComponent.MaxWalkSpeed` NewWalkSpeed (`self.CharacterMovement`)))

(fn `UserConstructionScript`)