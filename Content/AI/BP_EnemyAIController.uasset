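; Enemy AI controller that runs the character behavior tree and resolves directional melee attacks against the player.
; Perception tracks the tagged player in the blackboard, using a timer to delay losing sight.
; Left, right and up attacks notify the player controller, then compare directions: parry damages the AI, a later block check prevents player damage.
; At zero health the controller destroys itself, shortens its timings by level and spawns another enemy.
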(event `self.ReceiveBeginPlay`
  (bind _asbp_to_the_edge_player_controller (cast `/Game/BP_ToTheEdgePlayerController` (`GameplayStatics.GetPlayerController` 0)))
  (set `self.PlayerControllerReference` _asbp_to_the_edge_player_controller))

(event `self.ReceivePossess`
  (params (PossessedPawn :type "Pawn Object Reference"))
  (`self.RunBehaviorTree` "/Game/AI/BT_AICharacter.BT_AICharacter"))

(event `self.AIPerception.OnTargetPerceptionUpdated`
  (params (Actor :type "Actor Object Reference") (Stimulus :type "AIStimulus Structure"))
  (bind _blackboard (`self.Blackboard`))
  (if (and (`self.ActorHasTag` Actor "Player") (`.bSuccessfullySensed` (break `AIStimulus` Stimulus)))
    (`KismetSystemLibrary.PrintText` "I see you")
    (`KismetSystemLibrary.K2_ClearAndInvalidateTimerHandle` (`self.EnemyTimer`))
    (`BlackboardComponent.SetValueAsBool` _blackboard (`self.HasLineOfSight`) true)
    (`BlackboardComponent.SetValueAsObject` _blackboard (`self.PlayerActor`) Actor)
    (else
      (`KismetSystemLibrary.PrintText` "Where re you?")
      (bind _returnvalue (`KismetSystemLibrary.K2_SetTimerDelegate` (delegate `StartEnemyTimer`) (`self.LineOfSightTimer`)))
      (set `self.EnemyTimer` _returnvalue))))

(event `StartEnemyTimer`
  (bind _blackboard (`self.Blackboard`))
  (`BlackboardComponent.SetValueAsBool` _blackboard (`self.HasLineOfSight`) false)
  (`BlackboardComponent.SetValueAsObject` _blackboard (`self.PlayerActor`) null))

(event `AttackR`
  (bind _playercontrollerreference (`self.PlayerControllerReference`))
  (bind _attackdirection (`self.AttackDirection`))
  (bind _playercontrollerreference_2 (`self.PlayerControllerReference`))
  (bind _blockdirection (`/Game/BP_ToTheEdgePlayerController.BlockDirection` _playercontrollerreference))
  (`/Game/BP_ToTheEdgePlayerController.RightNotification` _playercontrollerreference)
  (`KismetSystemLibrary.Delay` (`self.ParryTime`) :!label _label)
  (bind _parried_ (`self.ParryCheck` _attackdirection _blockdirection))
  (if _parried_
    (bind _output_get (set `self.AIHealth` (- (`self.AIHealth`) (`/Game/BP_ToTheEdgePlayerController.AttackDamage` (`self.PlayerControllerReference`)))))
    (`KismetSystemLibrary.PrintString` (`KismetStringLibrary.Conv_DoubleToString` _output_get))
    (`self.AIHealthCheck`)
    (else
      (`KismetSystemLibrary.Delay` (- (`self.AttackTime`) (`self.ParryTime`)))
      (bind _blocked_ (`self.BlockCheck` _attackdirection _blockdirection))
      (if (not _blocked_)
        (bind _output_get_2 (set `/Game/BP_ToTheEdgePlayerController.Health` (- (`/Game/BP_ToTheEdgePlayerController.Health` _playercontrollerreference_2) (`self.AttackDamage`)) _playercontrollerreference_2))
        (`KismetSystemLibrary.PrintString` (`KismetStringLibrary.Conv_DoubleToString` _output_get_2))
        (`self.PlayerHealthCheck`)))))

(event `AttackL`
  (`/Game/BP_ToTheEdgePlayerController.LeftNotification` (`self.PlayerControllerReference`))
  (goto _label))

(event `AttackU`
  (`/Game/BP_ToTheEdgePlayerController.UpNotification` (`self.PlayerControllerReference`))
  (goto _label))

(event `LevelUp`
  (bind _output_get (set `self.LevelModifier` (+ (`self.Level`) (/ (`self.Level`) 10.0))))
  (`KismetSystemLibrary.PrintString` (`KismetStringLibrary.Conv_DoubleToString` _output_get))
  (bind _output_get_2 (set `self.AttackTime` (/ (`self.AttackTime`) (`self.LevelModifier`))))
  (`KismetSystemLibrary.PrintString` (`KismetStringLibrary.Conv_DoubleToString` _output_get_2))
  (bind _output_get_3 (set `self.ParryTIme` (/ (`self.ParryTIme`) (`self.LevelModifier`))))
  (`KismetSystemLibrary.PrintString` (`KismetStringLibrary.Conv_DoubleToString` _output_get_3)))

(event `self.ReceiveDestroyed`
  (`self.LevelUp`)
  (`AIBlueprintHelperLibrary.SpawnAIFromClass` "/Game/AI/BP_AICharacter.BP_AICharacter_C" "/Game/AI/BT_AICharacter.BT_AICharacter" (0.0 0.0 0.0) (struct) false null))

(fn `AIHealthCheck`
  (if (<= (`self.AIHealth`) 0.0)
    (`KismetSystemLibrary.PrintString` "FUCKED")
    (`self.K2_DestroyActor`)))

(fn `BlockCheck`
  (params (AttackDirection :type Integer) (BlockDirection :type Integer))
  (returns (`Blocked?` :type Boolean))
  (if (== AttackDirection BlockDirection)
    (`KismetSystemLibrary.PrintString` "BLOCKED!!")
    (return true)
    (else
      (return false))))

(fn `ParryCheck`
  (params (AttackDirection :type Integer) (BlockDirection :type Integer))
  (returns (`parried?` :type Boolean))
  (if (== AttackDirection BlockDirection)
    (`KismetSystemLibrary.PrintString` "PARRIED!!")
    (return true)
    (else
      (return false))))

(fn `PlayerHealthCheck`
  (bind _playercontrollerreference (`self.PlayerControllerReference`))
  (if (<= (`/Game/BP_ToTheEdgePlayerController.Health` _playercontrollerreference) 0.0)
    (`/Game/BP_ToTheEdgePlayerController.OnDeath` _playercontrollerreference)))

(fn `UserConstructionScript`)