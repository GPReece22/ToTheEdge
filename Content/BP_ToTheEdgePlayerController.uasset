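; Player controller for directional combat: creates the HUD, plays attack-direction and next-level animations on it, and handles player death.
; Left, Right and Up releases set BlockDirection, then block or slash depending on BlockTime, with input locked and Parryable set for BlockDelay.
; LevelIncrease raises difficulty by shrinking attack and parry times, gated by MaxSpeed.
; OnDeath unpossesses, fades out behind a death screen, then pauses and shows game over.
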(event `self.ReceiveBeginPlay`
  ;[1 1 1] Set up in game HUD
  (bind _returnvalue (`|CreateWidget` "/Game/HUD.HUD_C"))
  (bind _output_get (set `self.HUDReference` _returnvalue))
  (`UserWidget.AddToViewport` _output_get 0)
  ;[1 1 1] references the character to play animation
  (bind _asbp_to_the_edge_character (cast `/Game/BP_ToTheEdgeCharacter` (`self.K2_GetPawn`)))
  (set `self.PlayerPawnReferene` _asbp_to_the_edge_character))

(event `Key|Left`
  (params (Key :type "Key Structure"))
  ;[1 1 1] Take input from character and set block to that direction
  (:`Released`
    (`self.DisableInput` null)
    (set `self.BlockDirection` 1)
    (if (`self.BlockTime`)
      (`GameplayStatics.PlaySoundAtLocation` "/Game/Assets/Audio/block__1__Cue.block__1__Cue" (0.0 0.0 0.0) (struct) 1.0 1.0 0.0 null null null :!label _label)
      (`/Game/BP_ToTheEdgeCharacter.Block` (`self.PlayerPawnReferene`))
      (else
        (`/Game/BP_ToTheEdgeCharacter.left-Slash` (`self.PlayerPawnReferene`))))
    (set `self.Parryable` true :!label _label_2)
    (`KismetSystemLibrary.Delay` (`self.BlockDelay`))
    (`self.EnableInput` null)
    (set `self.Parryable` false)
    (set `self.BlockDirection` 7)))

(event `Key|Right`
  (params (Key :type "Key Structure"))
  ;[1 1 1] Take input from character and set block to that direction
  (:`Released`
    (`self.DisableInput` null)
    (set `self.BlockDirection` 2)
    (if (`self.BlockTime`)
      (goto _label)
      (else
        (`/Game/BP_ToTheEdgeCharacter.Right-Slash` (`self.PlayerPawnReferene`))
        (goto _label_2)))))

(event `Key|Up`
  (params (Key :type "Key Structure"))
  ;[1 1 1] Take input from character and set block to that direction
  (:`Released`
    (`self.DisableInput` null)
    (set `self.BlockDirection` 3)
    (if (`self.BlockTime`)
      (goto _label)
      (else
        (`/Game/BP_ToTheEdgeCharacter.left-Slash` (`self.PlayerPawnReferene`))
        (goto _label_2)))))

(event `OnDeath`
  (`self.UnPossess`)
  (`GameplayStatics.PlaySoundAtLocation` "/Game/Assets/Audio/Loss-Sound__1__Cue.Loss-Sound__1__Cue" (0.0 0.0 0.0) (struct) 1.0 1.0 0.0 null null null)
  (`PlayerCameraManager.StartCameraFade` :`self` (`self.PlayerCameraManager`) :`ToAlpha` 1.0 :`Duration` 3.0)
  (bind _returnvalue (`|CreateWidget` "/Game/WBP_DeathScreen.WBP_DeathScreen_C" self))
  (`UserWidget.AddToViewport` _returnvalue 0)
  (`KismetSystemLibrary.Delay` 3.0)
  (`GameplayStatics.SetGamePaused` true)
  (`WidgetLayoutLibrary.RemoveAllWidgets`)
  (bind _returnvalue_2 (`|CreateWidget` "/Game/WBP_GameOver.WBP_GameOver_C"))
  (`UserWidget.AddToViewport` _returnvalue_2 0)
  (set `PlayerController.bShowMouseCursor` true (`GameplayStatics.GetPlayerController` 0)))

(fn `LeftNotification`
  (bind _hudreference (`self.HUDReference`))
  (`UserWidget.PlayAnimation` _hudreference (`/Game/HUD.LeftAttackAnimation` _hudreference) 0.0 1 "Forward" 1.0 false))

(fn `Level increase`
  (bind _level (`self.Level`))
  ;[1 1 1] Decrease attack and parry windows by 1/level ratio each time
  (if (>= (`self.AttackTime`) (`self.MaxSpeed`))
    (set `self.Level` (+ _level 1.0))
    (set `self.Adjustment` (/ _level (`self.LevelRatio`)))
    (set `self.AttackTime` (- (`self.AttackTime`) (* (`self.AttackTime`) (`self.Adjustment`))))
    (set `self.ParryTime` (- (`self.ParryTime`) (* (`self.ParryTime`) (`self.Adjustment`))))))

(fn `NextLevelNotification`
  (bind _hudreference (`self.HUDReference`))
  (set `/Game/HUD.LoadScreenVisibility` "Visible" _hudreference)
  (`UserWidget.PlayAnimation` _hudreference (`/Game/HUD.NextLevelAnimation` _hudreference) 0.0 1 "Forward" 1.0 false))

(fn `RightNotification`
  (bind _hudreference (`self.HUDReference`))
  (`UserWidget.PlayAnimation` _hudreference (`/Game/HUD.RightAttackAnimation` _hudreference) 0.0 1 "Forward" 1.0 false))

(fn `UpNotification`
  (bind _hudreference (`self.HUDReference`))
  (`UserWidget.PlayAnimation` _hudreference (`/Game/HUD.UpAttackAnimation` _hudreference) 0.0 1 "Forward" 1.0 false))

(fn `UserConstructionScript`)