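; BP_Disintegration is a test actor, marked deprecated, that dissolves a skeletal mesh on a test input and then destroys itself.
; After a short delay, BeginPlay toggles mesh visibility and creates dynamic materials for armour and body.
; The input feeds the mesh's world location to both materials, then a timeline animates their dissolve amount and hardness.
; The construction script adds a Niagara component, which the graph never drives.
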(event `self.ReceiveBeginPlay`
  (bind _skeletalmesh (`self.SkeletalMesh`))
  ;[1 1 1] DEPRACTED
  (`KismetSystemLibrary.Delay` 2.0)
  (`SceneComponent.ToggleVisibility` (`self.SkeletalMesh`) false)
  (bind _returnvalue (`PrimitiveComponent.CreateDynamicMaterialInstance` _skeletalmesh 0 null "None"))
  (set `self.dmArmour` _returnvalue)
  (bind _returnvalue_2 (`PrimitiveComponent.CreateDynamicMaterialInstance` _skeletalmesh 1 null "None"))
  (set `self.dmBody` _returnvalue_2))

(event `InputAction|TestButton`
  (params (Key :type "Key Structure"))
  (bind _dmarmour (`self.dmArmour`))
  (bind _dmbody (`self.dmBody`))
  (bind _returnvalue (`KismetMathLibrary.Conv_VectorToLinearColor` (`SceneComponent.K2_GetComponentLocation` (`self.SkeletalMesh`))))
  ;[1 1 1] DEPRACTED
  (:`Pressed`
    (`/Engine/EditorBlueprintResources/StandardMacros.DoOnce` false
      (:`Completed`
        (`MaterialInstanceDynamic.SetVectorParameterValue` _dmarmour "Location" _returnvalue)
        (`MaterialInstanceDynamic.SetVectorParameterValue` _dmbody "Location" _returnvalue)
        (bind (_direction _dissolve_speed _hardness) (`Timeline|Dissolve` :!via `PlayFromStart`)
          (:`Update`
            (`MaterialInstanceDynamic.SetScalarParameterValue` _dmarmour "Amount" _dissolve_speed)
            (`MaterialInstanceDynamic.SetScalarParameterValue` _dmbody "Amount" _dissolve_speed)
            (`MaterialInstanceDynamic.SetScalarParameterValue` _dmarmour "Amount" _dissolve_speed)
            (`MaterialInstanceDynamic.SetScalarParameterValue` _dmbody "Hardness" _hardness)
            (`MaterialInstanceDynamic.SetScalarParameterValue` _dmarmour "Hardness" _hardness))
          (:`Finished`
            (`self.K2_DestroyActor`)))))))

(fn `UserConstructionScript`
  (`AddComponent|NODE_AddNiagaraComponent-1`))