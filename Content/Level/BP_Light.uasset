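; BP_Light is a flickering level light that spawns Niagara effects, apparently sparks, at randomized intervals.
; BeginPlay creates a dynamic fresnel material on the mesh and picks a random delay.
; Tick runs a DoOnce-gated loop: each delay spawns an effect and switches the material's Falloff between random low and fixed high values, then re-rolls the delay and re-arms.
; The node setting spark colour is unconnected.
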(event `self.ReceiveBeginPlay`
  (bind _returnvalue (`PrimitiveComponent.CreateDynamicMaterialInstance` (`self.StaticMesh`) 0 "/Game/Materials/M_FresnalLightBlue_Add_Inst.M_FresnalLightBlue_Add_Inst" "None"))
  (set `self.Material` _returnvalue)
  (set `self.randomSpawnTime` (`KismetMathLibrary.RandomFloatInRange` 0.25 2.0)))

(event `self.ReceiveTick`
  (params (DeltaSeconds :type "Float (single-precision)"))
  (bind _randomspawntime (`self.randomSpawnTime`))
  (if (`self.canSpawn`)
    (`/Engine/EditorBlueprintResources/StandardMacros.DoOnce` false :!label _label
      (:`Completed`
        (`KismetSystemLibrary.Delay` _randomspawntime)
        (`AddComponent|NODE_AddNiagaraComponent-0` :`RelativeTransform` (`SceneComponent.GetRelativeTransform` (`self.Scene1`)))
        (`MaterialInstanceDynamic.SetScalarParameterValue` (`self.Material`) "Falloff" (`KismetMathLibrary.RandomFloatInRange` 0.05 0.3))
        (`KismetSystemLibrary.Delay` _randomspawntime)
        (`AddComponent|NODE_AddNiagaraComponent-1` :`RelativeTransform` (`SceneComponent.GetRelativeTransform` (`self.Scene1`)))
        (`MaterialInstanceDynamic.SetScalarParameterValue` (`self.Material`) "Falloff" 30.0)
        (set `self.canSpawn` false)
        (set `self.randomSpawnTime` (`KismetMathLibrary.RandomFloatInRange` 0.25 2.0))))
    (else
      (set `self.canSpawn` true)
      (goto _label :!via `Reset`))))

(fn `UserConstructionScript`)